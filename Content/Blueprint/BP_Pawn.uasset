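; BP_Pawn is a flying pawn that constantly moves forward, steers with pitch and roll axis input, and fires rockets.
; Fire spawns a BP_Rocket at the Arrow transform, while UpDown and RightLeft apply frame-rate-independent local rotation.
; Boost caches FloatingPawnMovement acceleration and max speed, raises both through a Timeline lerp, then restores them on release without stopping the Timeline.
; Tick also prints current speed on screen.
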(event `InputAction|Fire`
  (params (Key :type "Key Structure"))
  ; Rocket 발사
  (:`Pressed`
    (`|SpawnActorFromClass` "/Game/Blueprint/BP_Rocket.BP_Rocket_C" (`SceneComponent.K2_GetComponentToWorld` (`self.Arrow`)) "AdjustIfPossibleButDontSpawnIfColliding" "MultiplyWithRoot" self self)))

(event `self.ReceiveTick`
  (params (DeltaSeconds :type "Float (single-precision)"))
  ; 전진
  (`self.AddMovementInput` (`self.GetActorForwardVector`))
  (`KismetSystemLibrary.PrintString` (`KismetStringLibrary.Conv_DoubleToString` (`KismetMathLibrary.VSize` (`self.GetVelocity`))) true true (struct :`G` 0.66 :`B` 1.0 :`A` 1.0) 0.0))

(event `InputAction|Boost`
  (params (Key :type "Key Structure"))
  ; Boost
  (:`Pressed`
    (set `self.RootAcceleration` (`FloatingPawnMovement.Acceleration` (`self.FloatingPawnMovement`)))
    (set `self.RootMaxSpeed` (`FloatingPawnMovement.MaxSpeed` (`self.FloatingPawnMovement`)))
    (`self.SpeedUpEvent`))
  (:`Released`
    (set `FloatingPawnMovement.Acceleration` (`self.RootAcceleration`) (`self.FloatingPawnMovement`))
    (set `FloatingPawnMovement.MaxSpeed` (`self.RootMaxSpeed`) (`self.FloatingPawnMovement`))))

(event `InputAxis|UpDown`
  (params (AxisValue :type "Float (single-precision)"))
  ; Pitch 회전
  (`self.K2_AddActorLocalRotation` (`KismetMathLibrary.MakeRotator` 0.0 (* AxisValue (`self.RotatorSpeed`) (`GameplayStatics.GetWorldDeltaSeconds`)))))

(event `InputAxis|RightLeft`
  (params (AxisValue :type "Float (single-precision)"))
  ; Roll 회전
  (`self.K2_AddActorLocalRotation` (`KismetMathLibrary.MakeRotator` (* AxisValue (`self.RotatorSpeed`) (`GameplayStatics.GetWorldDeltaSeconds`)))))

(event `SpeedUpEvent`
  (bind (_direction _alpha) (`Timeline|Timeline` :!via `PlayFromStart`)
    (:`Update`
      (set `FloatingPawnMovement.Acceleration` (`KismetMathLibrary.Lerp` (`self.RootAcceleration`) (`self.AccelerationUp`) _alpha) (`self.FloatingPawnMovement`))
      (set `FloatingPawnMovement.MaxSpeed` (`KismetMathLibrary.Lerp` (`self.RootMaxSpeed`) (`self.MaxSpeedUp`) _alpha) (`self.FloatingPawnMovement`)))))

(fn `UserConstructionScript`)