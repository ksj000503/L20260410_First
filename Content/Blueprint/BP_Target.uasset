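; BP_Target is a damageable objective actor whose destruction ends the game.
; On BeginPlay it caches the BP_GM game mode reference.
; AnyDamage subtracts damage from Hp, and at zero or below it destroys the actor and calls GameOver on the game mode.
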(event `self.ReceiveBeginPlay`
  (bind _asbp_gm (cast `/Game/Blueprint/BP_GM` (`GameplayStatics.GetGameMode`)))
  (set `self.As BP GM` _asbp_gm))

(event `self.ReceiveAnyDamage`
  (params (Damage :type "Float (single-precision)") (DamageType :type "DamageType Object Reference") (InstigatedBy :type "Controller Object Reference") (DamageCauser :type "Actor Object Reference"))
  ; 타겟 터지면 게임 종료
  (bind _output_get (set `self.Hp` (- (`self.Hp`) Damage)))
  (if (<= _output_get 0.0)
    (`self.K2_DestroyActor`)
    (`/Game/Blueprint/BP_GM.GameOver` (`self.As BP GM`))))

(fn `UserConstructionScript`)